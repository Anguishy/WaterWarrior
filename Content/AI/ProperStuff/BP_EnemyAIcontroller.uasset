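; AI controller for enemies that runs the BT_EnemyBase behavior tree and drives its state through the blackboard.
; On possess, after a short delay, it starts the tree, stores the player character in the blackboard and sets the roaming state.
; SetRoaming and SetFollowing write the corresponding E_States value to the state key.
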(event `self.ReceivePossess`
  (params (PossessedPawn :type "Pawn Object Reference"))
  (`KismetSystemLibrary.Delay` 0.2)
  (`self.RunBehaviorTree` "/Game/AI/ProperStuff/BT_EnemyBase.BT_EnemyBase")
  (`BlackboardComponent.SetValueAsObject` (`self.Blackboard`) (`self.Player Key Name`) (`GameplayStatics.GetPlayerCharacter` 0))
  (`self.SetRoaming`))

(fn `SetFollowing`
  (`BlackboardComponent.SetValueAsEnum` (`self.Blackboard`) (`self.State Key Name`) (enumliteral `/Game/AI/ProperStuff/E_States` "NewEnumerator1")))

(fn `SetRoaming`
  (`BlackboardComponent.SetValueAsEnum` (`self.Blackboard`) (`self.State Key Name`) (enumliteral `/Game/AI/ProperStuff/E_States` "NewEnumerator0")))

(fn `UserConstructionScript`)