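; BP_Alligator is an enemy AI that prioritizes eating radioactive spills, otherwise chasing and damaging the player or roaming.
; A delayed Tick takes the first BP_Spill found and moves to it through a resettable DoOnce, destroying it on arrival.
; Without a spill, it pursues a nearby player, subtracting Health on reaching them and triggering game over at zero.
; When the player is out of range, it moves to random reachable points.
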(event `self.ReceiveTick`
  (params (DeltaSeconds :type "Float (single-precision)"))
  (bind _targetspill (`self.TargetSpill`))
  ; Checks for spills of radioactive liquid, eats it then resumes chasing player
  (`KismetSystemLibrary.Delay` 0.5)
  (`self.FindSPill`)
  (`/Engine/EditorBlueprintResources/StandardMacros.IsValid` (`self.TargetSpill`)
    (:`Is Valid`
      (`/Engine/EditorBlueprintResources/StandardMacros.DoOnce` false :!label _label
        (:`Completed`
          (`|AIMoveTo` self (0.0 0.0 0.0) _targetspill 50.0
            (:`OnSuccess`
              (`self.K2_DestroyActor` _targetspill)
              (set `self.TargetSpill` null)
              (goto _label :!via `Reset`))
            (:`OnFail`
              (goto _label :!via `Reset`))))))
    (:`Is Not Valid`
      (if (< (`self.GetDistanceTo` (`GameplayStatics.GetPlayerCharacter` 0)) 1000.0)
        (`|AIMoveTo` self (0.0 0.0 0.0) (`GameplayStatics.GetPlayerCharacter` 0) 100.0
          (:`OnSuccess`
            (bind _asbp_third_person_character (cast `/Game/ThirdPerson/Blueprints/BP_ThirdPersonCharacter` (`GameplayStatics.GetPlayerCharacter` 0)))
            (bind _output_get (set `/Game/ThirdPerson/Blueprints/BP_ThirdPersonCharacter.Health` (- (`/Game/ThirdPerson/Blueprints/BP_ThirdPersonCharacter.Health` _asbp_third_person_character) 10.0) _asbp_third_person_character))
            (if (<= _output_get 0.0)
              (`/Game/ThirdPerson/Blueprints/BP_ThirdPersonCharacter.TriggerGameOver` _asbp_third_person_character))))
        (else
          (`KismetSystemLibrary.Delay` 0.2)
          (`self.Roaming`))))))

(event `FindSPill`
  ; looks for spill
  (bind _outactors (`GameplayStatics.GetAllActorsOfClass` "/Game/Blueprints/BP_Spill.BP_Spill_C"))
  (if (> (`KismetArrayLibrary.Array_Length` _outactors) 0)
    (set `self.TargetSpill` (`|GetArrayItem` _outactors))
    (else
      (set `self.TargetSpill` null))))

(event `Roaming`
  ; Roaming
  (`KismetSystemLibrary.Delay` 3.0)
  (`|AIMoveTo` self (`NavigationSystemV1.K2_GetRandomReachablePointInRadius` (`self.K2_GetActorLocation`) 2000.0 null null) null 100.0
    (:`OnSuccess`
      (`KismetSystemLibrary.Delay` 5.0))
    (:`OnFail`
      (`KismetSystemLibrary.Delay` 0.5))))

(fn `UserConstructionScript`)