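; BP_DeconUnit is a decontamination station that takes sludge from the player's held bucket and cleans it for score.
; Overlapping the interact zone with a filled bucket empties it into the unit, shows the liquid and enables input.
; Each E press reduces stored sludge, adds score and lerps a dynamic material's colour from green toward blue.
; Status text tracks progress, and input is disabled once the sludge is clean.
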(event `self.InteractZone.OnComponentBeginOverlap`
  (params (OverlappedComponent :type "PrimitiveComponent Object Reference") (OtherActor :type "Actor Object Reference") (OtherComp :type "PrimitiveComponent Object Reference") (OtherBodyIndex :type Integer) (bFromSweep :type Boolean) (SweepResult :type "HitResult Structure (by ref)"))
  (bind _statustxt (`self.StatusTxt`))
  (bind _asbp_third_person_character (cast `/Game/ThirdPerson/Blueprints/BP_ThirdPersonCharacter` OtherActor))
  (bind _heldbucketref (`/Game/ThirdPerson/Blueprints/BP_ThirdPersonCharacter.HeldBucketRef` _asbp_third_person_character))
  (bind _liquidlevel (`/Game/Blueprints/BP_Bucket.LiquidLevel` _heldbucketref))
  (if (> _liquidlevel 0.0)
    (bind _returnvalue (+ (`self.StoredSludge`) _liquidlevel))
    (set `self.StoredSludge` _returnvalue)
    (set `self.StartingSludge` _returnvalue)
    (set `/Game/Blueprints/BP_Bucket.LiquidLevel` 0.0 _heldbucketref)
    (`/Game/Blueprints/BP_Bucket.UpdateWaterVisuals` _heldbucketref)
    (`self.EnableInput` (`GameplayStatics.GetPlayerController` 0))
    (`TextRenderComponent.SetTextRenderColor` _statustxt (make `Color` 255 255 0 255))
    (`TextRenderComponent.K2_SetText` _statustxt (`KismetTextLibrary.Conv_StringToText` "Press E"))
    (`SceneComponent.SetRelativeScale3D` (`self.FluidLiquid`) (0.9 0.9 0.8))
    (`MaterialInstanceDynamic.SetVectorParameterValue` (`self.LiquidMaterialRef`) "FluidColour" (struct :`G` 1.0 :`A` 1.0))))

(event `Key|E`
  (params (Key :type "Key Structure"))
  (bind _statustxt (`self.StatusTxt`))
  (:`Pressed`
    (if (> (`self.StoredSludge`) 0.0)
      (set `self.StoredSludge` (- (`self.StoredSludge`) 0.2))
      (set `self.TotalScore` (+ (`self.TotalScore`) 10.0))
      (`MaterialInstanceDynamic.SetVectorParameterValue` (`self.LiquidMaterialRef`) "FluidColour" (`KismetMathLibrary.LinearColorLerp` (struct :`R` 0.015124 :`G` 0.110361 :`B` 0.557292 :`A` 0.263767) (struct :`G` 0.473958 :`A` 1.0) (/ (`self.StoredSludge`) (`self.StartingSludge`))))
      (`TextRenderComponent.K2_SetText` (`self.StatusTxt`) "Processing")
      (if (<= (`self.StoredSludge`) 0.0)
        (`TextRenderComponent.K2_SetText` _statustxt "Clean")
        (`TextRenderComponent.SetTextRenderColor` _statustxt (make `Color` 0 255 0 255))
        (`self.DisableInput` (`GameplayStatics.GetPlayerController` 0))))))

(fn `UserConstructionScript`
  (bind _returnvalue (`PrimitiveComponent.CreateDynamicMaterialInstance` (`self.FluidLiquid`) 0 null "None"))
  (set `self.LiquidMaterialRef` _returnvalue)
  (`SceneComponent.SetRelativeScale3D` (`self.FluidLiquid`) (0.9 0.9 0.0)))